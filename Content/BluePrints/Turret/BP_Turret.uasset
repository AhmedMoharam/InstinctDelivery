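; Turret actor that targets the player pawn while it is inside a trigger volume and fires BP_Projectile at it.
; Tick snaps the barrel toward the target and fires when a muzzle line trace within Range hits it and the cooldown allows.
; A looping FireRate timer, started and cleared on overlap, re-arms CanShoot.
; Shots fly along the muzzle rotation or, with UseSmartProjectile, toward SmartShooting's predicted target location.
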(event OnComponentBeginOverlap(TriggerVolume)
  (params (OverlappedComponent :type Primitive%20Component%20Object%20Reference) (OtherActor :type Actor%20Object%20Reference) (OtherComp :type Primitive%20Component%20Object%20Reference) (OtherBodyIndex :type Integer) (bFromSweep :type Boolean) (SweepResult :type Hit%20Result%20Structure%20%28by%20ref%29))
  (if (== OtherActor (Game|Player|GetPlayerPawn 0))
    ;[1 1 1] Set the Target and activate FireRate timer
    (if (not (Variables|TargetInfo|GetHasTarget))
      (Variables|TargetInfo|SetTargetPawn OtherActor)
      (Variables|TargetInfo|SetHasTarget true)
      (Variables|FireRate(Internal)|SetCanShoot true)
      (CallFunction|ActivateShootingTimer))))

(event OnComponentEndOverlap(TriggerVolume)
  (params (OverlappedComponent :type Primitive%20Component%20Object%20Reference) (OtherActor :type Actor%20Object%20Reference) (OtherComp :type Primitive%20Component%20Object%20Reference) (OtherBodyIndex :type Integer))
  (if (== OtherActor (Game|Player|GetPlayerPawn 0))
    ;[1 1 1] UnSet the target and Deactivate FireRate Timer
    (if (Variables|TargetInfo|GetHasTarget)
      (Variables|TargetInfo|SetHasTarget false)
      (CallFunction|DeactivateShootingTimer))))

(event Custom|SetCanShoot
  ;[1 1 1] Shooting Timer to handle Fire rate
  (Variables|FireRate(Internal)|SetCanShoot true))

(event Custom|ActivateShootingTimer
  ;[1 1 1] Shooting Timer to handle Fire rate
  (bind _returnvalue (Utilities|Time|SetTimerbyEvent (delegate Custom|SetCanShoot) (/ 1.0 (Variables|FiringSettings|GetFireRate)) true))
  (Variables|FireRate(Internal)|SetShootingTimerHandle _returnvalue))

(event Custom|DeactivateShootingTimer
  ;[1 1 1] Shooting Timer to handle Fire rate
  (Utilities|Time|ClearandInvalidateTimerbyHandle (Variables|FireRate(Internal)|GetShootingTimerHandle)))

(event EventBeginPlay)

(event Collision|EventActorBeginOverlap
  (params (OtherActor :type Actor%20Object%20Reference)))

(event EventTick
  (params (DeltaSeconds :type Float%20%28single-precision%29))
  (if (Variables|TargetInfo|GetHasTarget)
    ;[1 1 1] Get Target Location and Rotate Barrel to follow the target
    (Transformation|SetWorldRotation (Variables|Default|GetTurretBarrel) (Math|Rotator|MakeRotfromX (- (Transformation|GetActorLocation (Variables|TargetInfo|GetTargetPawn)) (Transformation|GetWorldLocation (Variables|Default|GetTurretBarrel)))) false false)
    ;[1 1 1] Shoot if target is in Range (have visual of target) && CanShoot depending on Firing Rate
    (bind _visible_ (CallFunction|IsTargetVisible))
    (if (and _visible_ (Variables|FireRate(Internal)|GetCanShoot))
      (if (Variables|FiringSettings|GetUseSmartProjectile)
        (CallFunction|FireSmartProjectile)
        (else
          (CallFunction|FireProjectile)))
      (Variables|FireRate(Internal)|SetCanShoot false))))

(fn ConstructionScript)

(fn IsTargetVisible
  (bind _turretbarrel (Variables|Default|GetTurretBarrel))
  (bind _returnvalue (Transformation|GetSocketTransform _turretbarrel "Muzzle" "RTS_World"))
  (bind _outhit (Collision|LineTraceByChannel (.location _returnvalue) (+ (.location _returnvalue) (* (Math|Rotator|GetRotationXVector (.rotation _returnvalue)) (Variables|FiringSettings|GetRange))) "TraceTypeQuery2" false 0 "ForOneFrame"))
  (return (== (.HitActor (Collision|BreakHitResult _outhit)) (Variables|TargetInfo|GetTargetPawn))))

(fn FireProjectile
  (bind _turretbarrel (Variables|Default|GetTurretBarrel))
  (Game|SpawnActorfromClass "/Game/BluePrints/Turret/BP_Projectile.BP_Projectile_C" (Math|Transform|MakeTransform (Transformation|GetSocketLocation _turretbarrel "Muzzle") (Transformation|GetSocketRotation _turretbarrel "Muzzle")) "Undefined" self 0))

(fn FireSmartProjectile
  (bind _turretbarrel (Variables|Default|GetTurretBarrel))
  (bind _returnvalue (Transformation|GetSocketLocation _turretbarrel "Muzzle"))
  (bind _tragetpredictedlocation (Class|SmartShootingComponent|PredictTargetLocation (Variables|Default|GetSmartShooting) (Variables|TargetInfo|GetTargetPawn) (Variables|FiringSettings|GetProjectileSpeed) _returnvalue))
  (Game|SpawnActorfromClass "/Game/BluePrints/Turret/BP_Projectile.BP_Projectile_C" (Math|Transform|MakeTransform _returnvalue (Math|Rotator|FindLookatRotation _returnvalue _tragetpredictedlocation)) "Undefined" self 0))