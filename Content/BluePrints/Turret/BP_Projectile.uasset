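; Projectile actor fired by BP_Turret that damages the player on overlap.
; The construction script casts its owner to BP_Turret and copies that turret's projectile speed into ProjectileMovement and its damage into the Damage variable.
; On overlap, it applies damage only when the other actor is the player pawn, and it does not destroy itself.
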(event EventBeginPlay)

(event Collision|EventActorBeginOverlap
  (params (OtherActor :type Actor%20Object%20Reference))
  (if (== OtherActor (Game|Player|GetPlayerPawn 0))
    (Game|Damage|ApplyDamage OtherActor (Variables|Default|GetDamage) 0 self)))

(fn ConstructionScript
  (bind _projectilemovement (Variables|Default|GetProjectileMovement))
  (bind _asbp_turret (Utilities|Casting|CastToBP_Turret (Components|GetOwner)))
  (Variables|/Script/Engine.ProjectileMovementComponent|SetInitialSpeed _projectilemovement (Variables|/Game/BluePrints/Turret/BP_Turret.BP_Turret_C|GetProjectileSpeed _asbp_turret))
  (Variables|/Script/Engine.ProjectileMovementComponent|SetMaxSpeed _projectilemovement (Variables|/Game/BluePrints/Turret/BP_Turret.BP_Turret_C|GetProjectileSpeed _asbp_turret))
  (Variables|Default|SetDamage (Variables|/Game/BluePrints/Turret/BP_Turret.BP_Turret_C|GetProjectileDamage _asbp_turret)))