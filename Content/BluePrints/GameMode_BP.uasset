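; Game mode for a grid-based ball game with turrets and coins, configured through a JsonConfigurator.
; GridManager builds the cell map, then supplies locations for the player start and configured turrets, whose cells are marked busy.
; Coins spawn on random available cells, add score when taken, and refill to the maximum below a threshold.
; It tracks player health from damage events, disables input at zero, and broadcasts health, score and death.
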(event Custom|CoinTaken
  ;[1 1 1] Coins Manager
  (Variables|Default|SetCoinsCount (- (Variables|Default|GetCoinsCount) 1))
  (bind _output_get (Variables|Default|SetScore (+ (Variables|Default|GetScore) (Variables|CoinsSettings|GetScorePerCoin))))
  (Default|CallScoreUpdate _output_get)
  (if (< (Variables|Default|GetCoinsCount) (Variables|CoinsSettings|GetCoinsGenerationThreshold))
    (CallFunction|GenerateCoins)))

(event Custom|GenerateCoins
  ;[1 1 1] Coins Manager
  (bind _cells (Class|GridManagerComponent|GetAvailableCells (Variables|Default|GetGridManager)))
  (while (< (Variables|Default|GetCoinsCount) (Variables|CoinsSettings|GetCoinsMaxCount))
    (bind _ascell_bp (Utilities|Casting|CastTocell_BP (Utilities|Array|Get(acopy) _cells (Math|Random|RandomIntegerinRange 0 (- (Utilities|Array|Length _cells) 1)))))
    (bind _spawnedactor (Default|SpawnItemsatRandomLocation _ascell_bp 1 "/Game/BluePrints/coin_BP.coin_BP_C"))
    (bind _ascoin_bp (Utilities|Casting|CastTocoin_BP _spawnedactor))
    (EventDispatchers|BindEventtoCoinTaken _ascoin_bp (delegate Custom|CoinTaken))
    (Variables|Default|SetCoinsCount (+ (Variables|Default|GetCoinsCount) 1))))

(event Custom|PlayerKilled
  ;[1 1 1] PlayerHealthSetup
  (Input|DisableInput (stale Custom|SpawnPlayer _asball_bp) (Game|GetPlayerController 0))
  (Default|CallPlayerKilledNotify))

(event Custom|ConstructMapGrid
  (bind _gridmanager (Variables|Default|GetGridManager))
  ;[1 1 1] Construct Map Using Cells
  (Variables|/Script/InstinctDelivery.GridManagerComponent|Setcell_class_name _gridmanager "/Game/BluePrints/cell_BP.cell_BP_C")
  (Variables|/Script/InstinctDelivery.GridManagerComponent|Setwall_class_name _gridmanager "/Game/BluePrints/Wall_BP.Wall_BP_C")
  (bind (_xcount _ycount) (Class|JsonConfigurator|GetGridSetup (Variables|Default|GetJsonConfigurator)))
  (Class|GridManagerComponent|ConstructCells (Variables|Default|GetGridManager) _xcount _ycount))

(event Custom|SpawnPlayer
  ;[1 1 1] Spawn Player at  required  Grid cell
  (bind (_xindex _yindex _yawangle) (Class|JsonConfigurator|GetPlayerStartPosition (Variables|Default|GetJsonConfigurator)))
  (bind _returnvalue (Class|GridManagerComponent|GetCellSpawnLocationatIndex (Variables|Default|GetGridManager) _xindex _yindex))
  (Transformation|SetActorLocationAndRotation (Game|Player|GetPlayerPawn 0) _returnvalue (Math|Rotator|MakeRotator 0.0 0.0 (Math|Conversions|ToFloat(Integer) _yawangle)))
  ;[1 1 1] PlayerHealthSetup
  (bind _playermaxhealth (Class|JsonConfigurator|GetPlayerMaxHealth (Variables|Default|GetJsonConfigurator)))
  (bind _output_get (Variables|Default|SetPlayerMaxHealth _playermaxhealth))
  (bind _output_get_2 (Variables|Default|SetPlayerHealth _output_get))
  (Default|CallHealthPercentageUpdate (/ _output_get_2 _output_get))
  (bind _asball_bp (Utilities|Casting|CastToBall_BP (Game|Player|GetPlayerPawn 0)))
  (EventDispatchers|BindEventtoPlayerDamaged _asball_bp (delegate Custom|PlayerDamaged)))

(event Custom|SetupCoins
  ;[1 1 1] Coins Setup
  (bind (_coinsmaxcount _coinsgenerationthreshold _scorepercoin) (Class|JsonConfigurator|GetCoinsSettings (Variables|Default|GetJsonConfigurator)))
  (Variables|CoinsSettings|SetCoinsMaxCount _coinsmaxcount)
  (Variables|CoinsSettings|SetCoinsGenerationThreshold _coinsgenerationthreshold)
  (Variables|CoinsSettings|SetScorePerCoin _scorepercoin)
  (CallFunction|GenerateCoins)
  (Default|CallScoreUpdate (Variables|Default|GetScore)))

(event Custom|SpawnAndConfigureTurrets
  (bind _gridmanager (Variables|Default|GetGridManager))
  ;[1 1 1] Spawn and Configure Turrets
  (bind _turretscount (Class|JsonConfigurator|GetTurretsCount (Variables|Default|GetJsonConfigurator)))
  (for _index (range 0 (- _turretscount 1))
    (bind (_xindex _yindex _yawangle _projectilespeed _firerate _range _usesmartprojectile _projectiledamage) (Class|JsonConfigurator|GetTurretSetupbyIndex (Variables|Default|GetJsonConfigurator) _index))
    (bind _returnvalue (Class|GridManagerComponent|GetCellSpawnLocationatIndex _gridmanager _xindex _yindex))
    (Class|GridManagerComponent|MarkCellBusy _gridmanager _xindex _yindex)
    (bind _returnvalue_2 (Game|SpawnActorfromClass "/Game/BluePrints/Turret/BP_Turret.BP_Turret_C" (Math|Transform|MakeTransform _returnvalue (Math|Rotator|MakeRotator 0.0 0.0 (Math|Conversions|ToFloat(Integer) _yawangle))) "Undefined" 0 0))
    (Variables|/Game/BluePrints/Turret/BP_Turret.BP_Turret_C|SetProjectileSpeed _returnvalue_2 _projectilespeed)
    (Variables|/Game/BluePrints/Turret/BP_Turret.BP_Turret_C|SetFireRate _returnvalue_2 _firerate)
    (Variables|/Game/BluePrints/Turret/BP_Turret.BP_Turret_C|SetRange _returnvalue_2 _range)
    (Variables|/Game/BluePrints/Turret/BP_Turret.BP_Turret_C|SetUseSmartProjectile _returnvalue_2 _usesmartprojectile)
    (Variables|/Game/BluePrints/Turret/BP_Turret.BP_Turret_C|SetProjectileDamage _returnvalue_2 _projectiledamage)))

(event Custom|PlayerDamaged
  (params (Damage :type Float%20%28single-precision%29))
  ;[1 1 1] PlayerHealthSetup
  (bind _output_get (Variables|Default|SetPlayerHealth (- (Variables|Default|GetPlayerHealth) Damage)))
  (Default|CallHealthPercentageUpdate (/ (Variables|Default|GetPlayerHealth) (Variables|Default|GetPlayerMaxHealth)))
  (if (<= _output_get 0.0)
    (CallFunction|PlayerKilled)))

(event EventBeginPlay)

(event EventTick
  (params (DeltaSeconds :type Float%20%28single-precision%29)))

(fn ConstructionScript)