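; Cell actor Blueprint that acts as a placeable level tile, exposing attachment points and an item spawn area.
; Marker components supply world transforms for the left and right neighbor cells and the four X/Y edges, plus a center spawn location.
; SpawnItemsAtRandomLocation spawns a given class inside the CoinSpawnArea box with random yaw, but returns inside its loop after the first spawn.
; The event graph and construction script are empty.
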(event EventBeginPlay)

(event Collision|EventActorBeginOverlap
  (params (OtherActor :type Actor%20Object%20Reference)))

(event EventTick
  (params (DeltaSeconds :type Float%20%28single-precision%29)))

(fn ConstructionScript)

(fn SpawnItemsatRandomLocation
  (params (Count :type Integer) (ActorClass :type Actor%20Class%20Reference))
  (bind _coinspawnarea (Variables|Default|GetCoinSpawnArea))
  (for _index (range 0 (- Count 1))
    (bind _returnvalue (Game|SpawnActorfromClass ActorClass (Math|Transform|MakeTransform (Math|Random|RandomPointinBoundingBox (Transformation|GetWorldLocation _coinspawnarea) (Components|Box|GetScaledBoxExtent _coinspawnarea)) (Math|Rotator|MakeRotator 0.0 0.0 (Math|Random|RandomFloatinRange 0.0 1.8e+02)) "1,1,1") "AdjustIfPossibleButAlwaysSpawn" 0 0))
    (return _returnvalue)))

(fn GetNextCelltoLeftTransform
  (return (Transformation|GetWorldTransform (Variables|Default|GetLeftCell))))

(fn GetNextCelltoRightTransform
  (return (Transformation|GetWorldTransform (Variables|Default|GetRightCell))))

(fn GetSpawnLocation
  (return (Transformation|GetWorldLocation (Variables|Default|GetCellCenterMarker))))

(fn GetXEdgeTransform
  (return (Transformation|GetWorldTransform (Variables|Default|GetXEdgeMarker))))

(fn GetXMinusEdgeTransform
  (return (Transformation|GetWorldTransform (Variables|Default|GetXMinusEdgeMarker))))

(fn GetYEdgeTransform
  (return (Transformation|GetWorldTransform (Variables|Default|GetYEdgeMarker))))

(fn GetYMinusEdgeTransform
  (return (Transformation|GetWorldTransform (Variables|Default|GetYMinusEdgeMarker))))