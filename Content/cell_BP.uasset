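; cell_BP is a level cell that exposes placement points for neighboring cells and edges, and can scatter coins inside itself.
; Getters return marker component transforms for the left and right neighbor cells and the four X/Y edges, plus a center spawn location.
; SpawnCoins adds a given number of child actor components at random points within the CoinSpawnArea box, each with random yaw.
; Its event graph and construction script are empty.
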(event EventBeginPlay)

(event Collision|EventActorBeginOverlap
  (params (OtherActor :type Actor%20Object%20Reference)))

(event EventTick
  (params (DeltaSeconds :type Float%20%28single-precision%29)))

(fn ConstructionScript)

(fn SpawnCoins
  (params (CoinsCount :type Integer))
  (bind _coinspawnarea (Variables|Default|GetCoinSpawnArea))
  (for _index (range 0 (- CoinsCount 1))
    (AddComponent|AddChildActorComponent false (Math|Transform|MakeTransform (Math|Random|RandomPointinBoundingBox (Variables|/Script/Engine.SceneComponent|GetRelativeLocation _coinspawnarea) (Components|Box|GetScaledBoxExtent _coinspawnarea)) (Math|Rotator|MakeRotator 0.0 0.0 (Math|Random|RandomFloatinRange 0.0 1.8e+02)) "1,1,1"))))

(fn GetNextCelltoLeftTransform
  (return (Transformation|GetWorldTransform (Variables|Default|GetLeftCell))))

(fn GetNextCelltoRightTransform
  (return (Transformation|GetWorldTransform (Variables|Default|GetRightCell))))

(fn GetSpawnLocation
  (return (Transformation|GetWorldLocation (Variables|Default|GetCellCenterMarker))))

(fn GetXEdgeTransform
  (return (Transformation|GetWorldTransform (Variables|Default|GetXEdgeMarker))))

(fn GetXMinusEdgeTransform
  (return (Transformation|GetWorldTransform (Variables|Default|GetXMinusEdgeMarker))))

(fn GetYEdgeTransform
  (return (Transformation|GetWorldTransform (Variables|Default|GetYEdgeMarker))))

(fn GetYMinusEdgeTransform
  (return (Transformation|GetWorldTransform (Variables|Default|GetYMinusEdgeMarker))))