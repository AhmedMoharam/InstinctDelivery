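; Ball Blueprint in the Character folder that reacts to being hit by projectiles.
; AnyDamage ignores causers other than BP_Projectile; for projectiles it applies knockback, destroys the projectile and broadcasts PlayerDamaged with the damage amount.
; DamageEffect pushes the Ball component along the projectile sphere's forward vector, scaling the impulse by projectile speed and DamageImpulseMultiplier.
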(event Custom|DamageEffect
  (params (DamageCauser :type BP%20Projectile%20Object%20Reference))
  (Physics|AddImpulse (Variables|Default|GetBall) (* (Math|Vector|GetForwardVector (Variables|/Game/BluePrints/Turret/BP_Projectile.BP_Projectile_C|GetSphere DamageCauser)) (* (Math|Vector|VectorLength (Transformation|GetVelocity DamageCauser)) (Variables|Default|GetDamageImpulseMultiplier))) "None" false))

(event EventBeginPlay)

(event EventTick
  (params (DeltaSeconds :type Float%20%28single-precision%29)))

(event Game|Damage|EventAnyDamage
  (params (Damage :type Float%20%28single-precision%29) (DamageType :type Damage%20Type%20Object%20Reference) (InstigatedBy :type Controller%20Object%20Reference) (DamageCauser :type Actor%20Object%20Reference))
  (bind _asbp_projectile (Utilities|Casting|CastToBP_Projectile DamageCauser))
  (CallFunction|DamageEffect _asbp_projectile)
  (Actor|DestroyActor _asbp_projectile)
  (Default|CallPlayerDamaged Damage))

(fn ConstructionScript)