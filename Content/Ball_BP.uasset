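; Ball_BP is a ball actor that currently has almost no active behavior.
; It enables input on BeginPlay, and its overlap event casts the other actor to BP_Projectile without acting on the result.
; Disconnected nodes would apply a large Y-axis force at the Ball component's center of mass, destroy the projectile and print the ball's speed, but none of them execute.
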(event EventBeginPlay
  (Input|EnableInput 0))

(event Collision|EventActorBeginOverlap
  (params (OtherActor :type Actor%20Object%20Reference))
  (bind _asbp_projectile (Utilities|Casting|CastToBP_Projectile OtherActor)))

(event EventTick
  (params (DeltaSeconds :type Float%20%28single-precision%29)))

(fn ConstructionScript)